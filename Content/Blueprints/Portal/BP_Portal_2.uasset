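; Linked pair of portals that show live views through each other, teleport overlapping actors and can be repositioned.
; Each tick, camera-position proxies drive the opposite scene captures' position, look-at rotation and distance-based FOV.
; Overlaps send JumpPortalMessage to exit at the other collider, with ExitCollider preventing an immediate bounce back.
; PlacePortal requires four dummy-portal edge traces to hit SurfaceType1, then moves the chosen portal and animates its scale.
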(event `self.ReceiveTick`
  (params (DeltaSeconds :type "Float (single-precision)"))
  (`self.UpdateCamera`))

(event `self.Col2.OnComponentBeginOverlap`
  (params (OverlappedComponent :type "PrimitiveComponent Object Reference") (OtherActor :type "Actor Object Reference") (OtherComp :type "PrimitiveComponent Object Reference") (OtherBodyIndex :type Integer) (bFromSweep :type Boolean) (SweepResult :type "HitResult Structure (by ref)"))
  (if (!= OverlappedComponent (`self.ExitCollider`))
    (bind _output_get (set `self.ExitCollider` (`self.Col1`)))
    (message `/Game/Blueprints/BPI_PortalJump.JumpPortal` OtherActor (+ (`SceneComponent.K2_GetComponentLocation` _output_get) (* (`SceneComponent.GetForwardVector` _output_get) 2.0)) (`SceneComponent.K2_GetComponentRotation` (`self.Capture1`)))))

(event `self.Col1.OnComponentBeginOverlap`
  (params (OverlappedComponent :type "PrimitiveComponent Object Reference") (OtherActor :type "Actor Object Reference") (OtherComp :type "PrimitiveComponent Object Reference") (OtherBodyIndex :type Integer) (bFromSweep :type Boolean) (SweepResult :type "HitResult Structure (by ref)"))
  (if (!= OverlappedComponent (`self.ExitCollider`))
    (bind _output_get (set `self.ExitCollider` (`self.Col2`)))
    (message `/Game/Blueprints/BPI_PortalJump.JumpPortal` OtherActor (+ (`SceneComponent.K2_GetComponentLocation` _output_get) (* (`SceneComponent.GetForwardVector` _output_get) 2.0)) (`SceneComponent.K2_GetComponentRotation` (`self.Capture2`)))))

(event `self.Col2.OnComponentEndOverlap`
  (params (OverlappedComponent :type "PrimitiveComponent Object Reference") (OtherActor :type "Actor Object Reference") (OtherComp :type "PrimitiveComponent Object Reference") (OtherBodyIndex :type Integer))
  (if (== OverlappedComponent (`self.ExitCollider`))
    (set `self.ExitCollider` null)))

(event `self.Col1.OnComponentEndOverlap`
  (params (OverlappedComponent :type "PrimitiveComponent Object Reference") (OtherActor :type "Actor Object Reference") (OtherComp :type "PrimitiveComponent Object Reference") (OtherBodyIndex :type Integer))
  (if (== OverlappedComponent (`self.ExitCollider`))
    (set `self.ExitCollider` null)))

(event `PlacePortal`
  (params (`Red/Blue` :type Boolean) (NewLocation :type "Vector Structure") (NewRotation :type "Rotator Structure"))
  (bind _returnvalue (select `bool` `Red/Blue` :`false` (`self.D1`) :`true` (`self.D2`)))
  (`self.CanPlacePortal` NewLocation NewRotation
    (:`Can Place`
      (`SceneComponent.SetRelativeScale3D` _returnvalue (0.1 0.1 0.1))
      (`SceneComponent.K2_SetWorldLocationAndRotation` _returnvalue NewLocation NewRotation false false)
      (bind (_direction _scale) (`Timeline|Scale` :!via `PlayFromStart`)
        (:`Update`
          (`SceneComponent.SetRelativeScale3D` _returnvalue (`KismetMathLibrary.Conv_DoubleToVector` _scale)))))))

(fn `CheckSurface`
  (params (Side :type "SceneComponent Object Reference"))
  (returns (ReturnValue :type Boolean))
  (bind _returnvalue (`SceneComponent.K2_GetComponentLocation` Side))
  (bind (_outhit _returnvalue_2) (`KismetSystemLibrary.LineTraceSingle` _returnvalue (+ _returnvalue (* (`SceneComponent.GetForwardVector` Side) 50.0)) "TraceTypeQuery1"))
  (if _returnvalue_2
    (return (`|EnumEquality` (`PhysicalMaterial.SurfaceType` (`.PhysMat` (`GameplayStatics.BreakHitResult` _outhit))) "SurfaceType1"))
    (else
      (return false))))

(fn `UpdateCamera`
  (`SceneComponent.K2_SetWorldLocation` (`self.PSim02`) (`PlayerCameraManager.GetCameraLocation` (`GameplayStatics.GetPlayerCameraManager` 0)) false false)
  (`SceneComponent.K2_SetWorldLocation` (`self.PSim01`) (`PlayerCameraManager.GetCameraLocation` (`GameplayStatics.GetPlayerCameraManager` 0)) false false)
  (`self.UpdateCapture` (`self.Capture1`) (`SceneComponent.RelativeLocation` (`self.PSim02`)))
  (`self.UpdateCapture` (`self.Capture2`) (`SceneComponent.RelativeLocation` (`self.PSim01`)))
  (return))

(fn `UserConstructionScript`)