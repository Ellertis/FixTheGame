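; BP_ToFocus is a one-shot trigger actor that plays a cutscene when the player overlaps it.
; On overlap it starts the referenced Cutscene's sequence player and waits for the sequence's duration.
; It then sets the Cinematic flag to true on the Singleton game instance and destroys itself, skipping both if that cast fails.
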(event `self.ReceiveActorBeginOverlap`
  (params (OtherActor :type "Actor Object Reference"))
  (bind _sequenceplayer (`LevelSequenceActor.SequencePlayer` (`self.Cutscene`)))
  (if (== OtherActor (`/Game/Blueprints/BFL_Main.MyPlayer`))
    (`MovieSceneSequencePlayer.Play` _sequenceplayer)
    (`KismetSystemLibrary.Delay` (`TimeManagementBlueprintLibrary.Conv_QualifiedFrameTimeToSeconds` (`MovieSceneSequencePlayer.GetDuration` _sequenceplayer)))
    (bind _assingleton (cast `/Game/Blueprints/Singleton` (`GameplayStatics.GetGameInstance`)))
    (set `/Game/Blueprints/Singleton.Cinematic` true _assingleton)
    (`self.K2_DestroyActor`)))

(fn `UserConstructionScript`)