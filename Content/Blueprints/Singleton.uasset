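; Singleton Blueprint that holds the player's health state for the game.
; DealDamage subtracts the given amount from PlayerHP without clamping it.
; IsPlayerAlive sets the PlayerAlive flag from whether PlayerHP is above zero and returns it, so the flag refreshes only when that function is called.
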(fn `DealDamage`
  (params (Damage :type Integer))
  (set `self.PlayerHP` (- (`self.PlayerHP`) Damage)))

(fn `IsPlayerAlive`
  (returns (PlayerStatus :type Boolean))
  (if (> (`self.PlayerHP`) 0)
    (set `self.PlayerAlive?` true)
    (else
      (set `self.PlayerAlive?` false)))
  (return (`self.PlayerAlive?`)))